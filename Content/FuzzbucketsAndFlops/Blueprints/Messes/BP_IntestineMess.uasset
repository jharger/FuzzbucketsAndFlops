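; BP_IntestineMess is an intestine mess actor that randomizes its appearance in the construction script, with no active event logic.
; After running the parent construction script, it picks a random base mesh from Meshes and gives it a random yaw.
; It then attaches a random number of IntestineDetailA mesh components in a ring just inside the base mesh's bounds radius, each with random yaw and horizontal scale.
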(event EventBeginPlay)

(event Collision|EventActorBeginOverlap
  (params (OtherActor :type Actor%20Object%20Reference)))

(event EventTick
  (params (DeltaSeconds :type Float%20%28single-precision%29)))

(fn ConstructionScript
  (|CallParentFunction)
  (Components|StaticMesh|SetStaticMesh (Variables|Default|GetStaticMesh) (.OutItem (Utilities|Array|Random (Variables|Default|GetMeshes))))
  (Transformation|SetRelativeRotation (Variables|Default|GetStaticMesh) (Math|Rotator|MakeRotator 0.0 0.0 (Math|Random|RandomFloatinRange 0.0 3.6e+02)) false false)
  (for _index (range 0 (Math|Random|RandomIntegerinRange (Variables|Default|GetMinDetails) (Variables|Default|GetMaxDetails)))
    (bind _returnvalue (AddComponent|AddStaticMeshComponent true (Math|Transform|MakeTransform (* (Math|Vector|RotateVector (Class|KismetMathLibrary|VectorForward) (Math|Rotator|MakeRotator 0.0 0.0 (Math|Random|RandomFloatinRange 0.0 3.6e+02))) (* (.SphereRadius (Collision|GetComponentBounds (Variables|Default|GetStaticMesh))) 0.8)) (Math|Rotator|MakeRotator 0.0 0.0 (Math|Random|RandomFloatinRange 0.0 3.6e+02)) (Math|Vector|MakeVector (Math|Random|RandomFloatinRange 0.8 1.2) (Math|Random|RandomFloatinRange 0.8 1.2) 1.0))))
    (Components|StaticMesh|SetStaticMesh _returnvalue "/Game/Assets/Entrails/IntestineDetailA.IntestineDetailA")
    (Transformation|AttachComponentToComponent _returnvalue (Variables|Default|GetStaticMesh) "None" "KeepRelative" "KeepRelative" "KeepRelative" true)))