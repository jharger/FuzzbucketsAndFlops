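; BP_MessCounter tracks how much mess remains in the level and triggers the win screen once enough is cleared.
; On BeginPlay it stores the count of actors implementing BPI_InteractableInterface as the mess total.
; Every Tick it re-queries and recounts those actors, then opens WinScreenMap when the remaining fraction falls to GoalPercent or below.
; Every implementer of that interface counts as mess, with no further filtering.
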(event EventTick
  (params (DeltaSeconds :type Float%20%28single-precision%29))
  (bind _outactors (Actor|GetAllActorswithInterface "/Game/FuzzbucketsAndFlops/Blueprints/Messes/BPI_InteractableInterface.BPI_InteractableInterface_C"))
  (bind _output_get (Variables|Default|SetcurrentMess (Utilities|Array|Length _outactors)))
  (if (<= (Math|Float|SafeDivide (Math|Conversions|ToFloat(Integer) _output_get) (Math|Conversions|ToFloat(Integer) (stale EventBeginPlay _output_get))) (Variables|Default|GetgoalPercent))
    (Game|OpenLevel(byName) "WinScreenMap")))

(event EventBeginPlay
  (bind _outactors (Actor|GetAllActorswithInterface "/Game/FuzzbucketsAndFlops/Blueprints/Messes/BPI_InteractableInterface.BPI_InteractableInterface_C"))
  (bind _output_get (Variables|Default|SettotalMess (Utilities|Array|Length _outactors))))

(fn ConstructionScript)