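; Fuzzbucket rabbit pawn that takes move orders and passes them to its controller.
; BeginPlay configures its FloatingPawnMovement, and OrdertoLocation forwards the target location to a valid controller as an interface message.
; Helper functions fetch the first BP_Target's location and find the interactable nearest the stored command location within a maximum distance.
; Older AIMoveTo and closest-interactable logic remains disconnected in the event graph.
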(event EventBeginPlay
  (bind _floatingpawnmovement (Variables|Default|GetFloatingPawnMovement))
  (Variables|/Script/Engine.FloatingPawnMovement|SetMaxSpeed _floatingpawnmovement (Variables|Default|GetfMOVE_SPEED))
  (Variables|/Script/Engine.FloatingPawnMovement|SetAcceleration _floatingpawnmovement (Variables|Default|GetfACCEL_SPEED))
  (Variables|/Script/Engine.FloatingPawnMovement|SetDeceleration _floatingpawnmovement (Variables|Default|GetfDECEL_SPEED)))

(event EventOrdertoLocation
  (params (TargetLocation :type Vector :default "0, 0, 0"))
  (bind _returnvalue (Pawn|GetController))
  (Utilities|IsValid _returnvalue
    (:Is%20Valid
      (Class|BPICommandable|OrdertoLocation(Message) _returnvalue TargetLocation))))

(event EventTick
  (params (DeltaSeconds :type Float%20%28single-precision%29)))

(fn ConstructionScript)

(fn GetTarget
  (bind _outactors (Actor|GetAllActorsOfClass "/Game/FuzzbucketsAndFlops/Blueprints/Player/BP_Target.BP_Target_C"))
  (for (_array_element _array_index) _outactors ; Find first instance of BP_Target
    ;[0.2157 0.6379 1] For each BP_Target (There should only be one)
    (if (== _array_index 0)
      (return (Transformation|GetActorLocation _array_element) (!= (Utilities|Array|Length _outactors) 0))))
  (return (Transformation|GetActorLocation _array_element) (!= (Utilities|Array|Length _outactors) 0)))

(fn GetMess
  (bind _outactors (Actor|GetAllActorswithInterface "/Game/FuzzbucketsAndFlops/Blueprints/Messes/BPI_InteractableInterface.BPI_InteractableInterface_C"))
  (Variables|Default|SetfClosest (Variables|Default|GetfMAX_CMD_DIST))
  (Variables|Default|SetaClosest 0) ; Setting to None
  (for _array_element _outactors
    ;[0.2157 0.6379 1] For Each Interactable
    (if (< (Math|Vector|Distance(Vector) (Variables|Default|GetvCmdLoc) (Transformation|GetActorLocation _array_element)) (Variables|Default|GetfClosest))
      (Variables|Default|SetfClosest (Math|Vector|Distance(Vector) (Variables|Default|GetvCmdLoc) (Transformation|GetActorLocation _array_element)))
      (Variables|Default|SetaClosest _array_element)))
  (return (Variables|Default|GetaClosest)))