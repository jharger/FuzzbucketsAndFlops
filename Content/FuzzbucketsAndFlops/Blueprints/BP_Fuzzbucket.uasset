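; BP_Fuzzbucket is an actor that, on BeginPlay, looks for the interactable closest to the level's command target.
; It takes the first BP_Target's location as the command point, then linearly scans all BPI_InteractableInterface actors for the nearest within FMAXCMDDIST.
; Results only print to screen: each distance, then the winner's name or a not-found message.
; Overlap, Tick and the construction script are empty.
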(event EventBeginPlay
  (bind _outactors (Actor|GetAllActorsOfClass "/Game/FuzzbucketsAndFlops/Blueprints/Player/BP_Target.BP_Target_C"))
  (for (_array_element _array_index) _outactors ; Find first instance of BP_Target
    ;[0.2157 0.6379 1] For each BP_Target (There should only be one
    (if (== _array_index 0)
      (Variables|Default|SetvCmdLoc (Transformation|GetActorLocation _array_element))))
  (bind _outactors_2 (Actor|GetAllActorswithInterface "/Game/FuzzbucketsAndFlops/Blueprints/BPI_InteractableInterface.BPI_InteractableInterface_C"))
  (Variables|Default|SetfClosest (Variables|Default|GetfMAX_CMD_DIST))
  (Variables|Default|SetaClosest 0) ; Setting to None
  (for (_array_element_2 _array_index_2) _outactors_2
    ;[0.2157 0.6379 1] For Each Interactable
    (Development|PrintString (Utilities|String|Append (Utilities|String|Append (Utilities|String|ToString(Integer) _array_index_2) ": ") (Utilities|String|ToString(Float) (Math|Vector|Distance(Vector) (Variables|Default|GetvCmdLoc) (Transformation|GetActorLocation _array_element_2)))))
    (if (< (Math|Vector|Distance(Vector) (Variables|Default|GetvCmdLoc) (Transformation|GetActorLocation _array_element_2)) (Variables|Default|GetfClosest))
      (Variables|Default|SetfClosest (Math|Vector|Distance(Vector) (Variables|Default|GetvCmdLoc) (Transformation|GetActorLocation _array_element_2)))
      (Variables|Default|SetaClosest _array_element_2)))
  (if (!= (Variables|Default|GetaClosest) 0)
    (Development|PrintString (Utilities|GetDisplayName (Variables|Default|GetaClosest)))
    (else
      (Development|PrintString "NOT FOUND!"))))

(event Collision|EventActorBeginOverlap
  (params (OtherActor :type Actor%20Object%20Reference)))

(event EventTick
  (params (DeltaSeconds :type Float%20%28single-precision%29)))

(fn ConstructionScript)